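; Player controller that handles pausing the game and showing the pause menu.
; On BeginPlay it creates and stores a pause menu widget for player 0.
; The IA_Pause input calls CustomPause, which toggles the game's paused state.
; When paused it shows the widget with UI-only input and cursor; otherwise it restores game-only input, hides the cursor and removes the widget.
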(event `self.ReceiveBeginPlay`
  (bind _returnvalue (`|CreateWidget` "/Game/IkeaBlueprints/Widgets/WB_PauseMenu.WB_PauseMenu_C" (`GameplayStatics.GetPlayerController` 0)))
  (set `self.PauseWidget` _returnvalue))

(event `CustomPause`
  (bind _returnvalue (`GameplayStatics.IsGamePaused`))
  (bind _pausewidget (`self.PauseWidget`))
  (bind _pausewidget_2 (`self.PauseWidget`))
  (`GameplayStatics.SetGamePaused` (not _returnvalue))
  (if _returnvalue
    (`UserWidget.AddToViewport` _pausewidget_2 0)
    (`WidgetBlueprintLibrary.SetInputMode_UIOnlyEx` self _pausewidget_2)
    (set `self.bShowMouseCursor` true)
    (else
      (`/Engine/EditorBlueprintResources/StandardMacros.IsValid` _pausewidget
        (:`Is Valid`
          (`WidgetBlueprintLibrary.SetInputMode_GameOnly` self)
          (set `self.bShowMouseCursor` false)
          (`Widget.RemoveFromParent` _pausewidget))))))

(event `EnhancedInput|/Game/ThirdPerson/Input/Actions/IA_Pause`
  (params (ActionValue :type Boolean) (ElapsedSeconds :type "Float (double-precision)") (TriggeredSeconds :type "Float (double-precision)") (InputAction :type "InputAction Object Reference" :default "/Game/ThirdPerson/Input/Actions/IA_Pause.IA_Pause"))
  (:`Triggered`
    (`self.CustomPause`)))

(fn `UserConstructionScript`)