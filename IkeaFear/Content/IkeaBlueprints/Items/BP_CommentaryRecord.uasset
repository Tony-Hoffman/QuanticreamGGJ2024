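; Pickup commentary record that, on player overlap, disables its collision, hides itself and starts developer-configured voice commentary with subtitles.
; Parallel subtitle and audio arrays are length-checked, with debug prints when either is empty or their sizes differ.
; An event-driven loop increments an index, then either shows that subtitle and spawns its 2D sound or removes the widget.
; Each sound's finished event re-enters the loop.
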(event `self.ReceiveBeginPlay`
  (if (== (`KismetArrayLibrary.Array_Length` (`self.VoiceClipStrings`)) (`KismetArrayLibrary.Array_Length` (`self.VoiceClipAudio`)))
    (set `self.EqualLengthArrays` true)
    (else
      (set `self.EqualLengthArrays` false))))

(event `self.CollisionVolume.OnComponentBeginOverlap`
  (params (OverlappedComponent :type "PrimitiveComponent Object Reference") (OtherActor :type "Actor Object Reference") (OtherComp :type "PrimitiveComponent Object Reference") (OtherBodyIndex :type Integer) (bFromSweep :type Boolean) (SweepResult :type "HitResult Structure (by ref)"))
  (if (== OtherActor (`GameplayStatics.GetPlayerCharacter` 0))
    (`PrimitiveComponent.SetCollisionEnabled` (`self.CollisionVolume`) "NoCollision")
    (`SceneComponent.SetVisibility` (`self.RecordItem`) false false)
    (if (not (== (`KismetArrayLibrary.Array_Length` (`self.VoiceClipStrings`)) 0))
      (if (not (== (`KismetArrayLibrary.Array_Length` (`self.VoiceClipAudio`)) 0))
        (if (`self.EqualLengthArrays`)
          (`self.CreateSubtitleWidget`)
          (`self.PlayCommentaryLoop`)
          (else
            (`KismetSystemLibrary.PrintString` "CANNOT PLAY COMMENTARY - UNEQUAL STRING/AUDIO LENGTH ARRAYS")))
        (else
          (`KismetSystemLibrary.PrintString` "COMMENTARY AUDIO ARRAY LENGTH 0")))
      (else
        (`KismetSystemLibrary.PrintString` "COMMENTARY STRING ARRAY LENGTH 0")))))

(event `PlayCommentaryLoop`
  (bind _result (`/Engine/EditorBlueprintResources/StandardMacros.IncrementInt` (`self.CurrentSoundInt`))
    (:`  `
      (if (<= (`KismetArrayLibrary.Array_Length` (`self.VoiceClipStrings`)) (+ _result 1))
        (`self.PlayCommentarySegment`)
        (else
          (`Widget.RemoveFromParent` (`self.SubtitleWidget`)))))))

(event `PlayCommentarySegment`
  (bind _currentsoundint (`self.CurrentSoundInt`))
  (`/Game/IkeaBlueprints/Widgets/WB_CommentarySubtitle.SetSubtitleText` (`self.SubtitleWidget`) (`|GetArrayItem` (`self.VoiceClipStrings`) _currentsoundint))
  (bind _returnvalue (`GameplayStatics.SpawnSound2D` (`|GetArrayItem` (`self.VoiceClipAudio`) _currentsoundint) 1.0 1.0 0.0 null))
  (add `AudioComponent.OnAudioFinished` _returnvalue (delegate `OnAudioSegmentEnd`)))

(event `OnAudioSegmentEnd`
  (`self.PlayCommentaryLoop`))

(fn `CreateSubtitleWidget`
  (bind _returnvalue (`|CreateWidget` "/Game/IkeaBlueprints/Widgets/WB_CommentarySubtitle.WB_CommentarySubtitle_C" (`GameplayStatics.GetPlayerController` 0)))
  (bind _output_get (set `self.SubtitleWidget` _returnvalue))
  (`UserWidget.AddToViewport` _output_get 0))

(fn `UserConstructionScript`)