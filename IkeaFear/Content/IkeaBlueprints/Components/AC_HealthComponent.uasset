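; Health component for the player character or enemy AI, tracking current health, damage, full heals and death.
; BeginPlay casts the owner to flag player or enemy and fills health to max.
; Damage sets a dead flag at zero and prints debug health.
; Death is deferred to HandlePostDialogue, which routes through Die to player or enemy death events, both currently empty stubs.
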(event `self.ReceiveBeginPlay`
  (bind _returnvalue (`self.GetOwner`))
  (bind _asbp_third_person_character (cast `/Game/ThirdPerson/Blueprints/BP_ThirdPersonCharacter` _returnvalue)
    (:`then`
      (set `self.PlayerBP` _asbp_third_person_character)
      (set `self.IsPlayer?` true))
    (:`CastFailed`
      (bind _asbp_enemy_ai_parent (cast `/Game/StealthAI/EnemyAI/BP_EnemyAI_PARENT` _returnvalue))
      (set `self.EnemyBP` _asbp_enemy_ai_parent)
      (set `self.IsPlayer?` false)))
  (set `self.CurrHealth` (`self.MaxHealth`)))

(event `FullHeal`
  (set `self.CurrHealth` (`self.MaxHealth`)))

(event `TakeDamage`
  (params (DamageTaken :type Integer))
  (set `self.CurrHealth` (- (`self.CurrHealth`) DamageTaken))
  (`self.CheckDeath`)
  (`self.PrintHealthDebug`))

(event `CheckDeath`
  (if (<= (`self.CurrHealth`) 0)
    (set `self.IsDead?` true)))

(event `HandlePostDialogue`
  (if (`self.IsDead?`)
    (`self.Die`)))

(event `Die`
  (if (`self.IsPlayer?`)
    (`self.PlayerDeath`)
    (else
      (`self.EnemyDeath`))))

(event `PlayerDeath`)

(event `EnemyDeath`)

(fn `PrintHealthDebug`
  (`KismetSystemLibrary.PrintString` (`self.GetDebugHealthString`)))