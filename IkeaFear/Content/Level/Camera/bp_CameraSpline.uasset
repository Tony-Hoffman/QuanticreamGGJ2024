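; Spline camera actor that takes over the player's view and tracks the player along a spline.
; Player overlap with SplineCollision sets Active, which this Blueprint never clears.
; While active, Tick eases SplineCamera toward the spline point nearest the player using VInterpTo.
; Every such tick also re-sets the actor as view target and passes the camera to the player character via UpdateCameraComponentMessage.
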(event `self.SplineCollision.OnComponentBeginOverlap`
  (params (OverlappedComponent :type "PrimitiveComponent Object Reference") (OtherActor :type "Actor Object Reference") (OtherComp :type "PrimitiveComponent Object Reference") (OtherBodyIndex :type Integer) (bFromSweep :type Boolean) (SweepResult :type "HitResult Structure (by ref)"))
  ;[1 1 1] Setting Camera to Active on Box Trigger Overlap
  (if (== (`GameplayStatics.GetPlayerCharacter` 0) OtherActor)
    (set `self.Active` true)))

(event `self.ReceiveTick`
  (params (DeltaSeconds :type "Float (single-precision)"))
  ;[1 1 1] Camera Following Spline when Set to Active
  (if (`self.Active`)
    (`SceneComponent.K2_SetWorldLocation` (`self.SplineCamera`) (`KismetMathLibrary.VInterpTo` (`SceneComponent.K2_GetComponentLocation` (`self.SplineCamera`)) (`SplineComponent.FindLocationClosestToWorldLocation` (`self.Spline`) (`self.GetPlayerWorldLoc`) "World") (`GameplayStatics.GetWorldDeltaSeconds`) 2.0) false false)
    (`PlayerController.SetViewTargetWithBlend` (`GameplayStatics.GetPlayerController` 0) self 0.0 "VTBlend_Linear" 0.0 false)
    (message `/Game/Level/BPI_Player.UpdateCameraComponent` (`GameplayStatics.GetPlayerCharacter` 0) (`self.SplineCamera`))))

(fn `UserConstructionScript`)