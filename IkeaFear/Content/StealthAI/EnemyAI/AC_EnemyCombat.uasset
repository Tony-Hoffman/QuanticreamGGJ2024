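; Enemy AI combat component that starts a dialogue encounter when the player is within grabbing range.
; ChaseUpdate checks range, then StartDialogue freezes movement and, through a DoOnce, switches to the enemy's dialogue camera, shows WB_DialogueCombat and hides the player mesh.
; EndDialogue restores movement, camera, input and visibility.
; UpdateDialogue is empty, and the distance comparison in IsWithinGrabbingDistance is left unconnected.
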(event `self.ReceiveBeginPlay`
  (bind _asbp_enemy_ai_parent (cast `/Game/StealthAI/EnemyAI/BP_EnemyAI_PARENT` (`self.GetOwner`)))
  (set `self.ThisEnemy` _asbp_enemy_ai_parent)
  (bind _asbp_third_person_character (cast `/Game/ThirdPerson/Blueprints/BP_ThirdPersonCharacter` (`GameplayStatics.GetPlayerCharacter` 0)))
  (set `self.Player` _asbp_third_person_character)
  (`KismetSystemLibrary.PrintString` "End of EnemyCombat Init"))

(event `ChaseUpdate`
  (if (`self.IsWithinGrabbingDistance`)
    (`self.StartDialogue`)
    (`self.UpdateDialogue`)))

(event `StartDialogue`
  (bind _player (`self.Player`))
  (bind _player_2 (`self.Player`))
  (bind _returnvalue (`Pawn.GetLocalViewingPlayerController` _player_2))
  (bind _dialoguecamera (`/Game/StealthAI/EnemyAI/BP_EnemyAI_PARENT.DialogueCamera` (`self.ThisEnemy`)))
  (`CharacterMovementComponent.DisableMovement` (`Character.CharacterMovement` (`self.Player`)))
  (`/Engine/EditorBlueprintResources/StandardMacros.DoOnce` false
    (:`Completed`
      (`self.SetActive` (`/Game/ThirdPerson/Blueprints/BP_ThirdPersonCharacter.FollowCamera` _player) false false)
      (`self.SetActive` _dialoguecamera true false)
      (`Controller.SetControlRotation` (`Pawn.GetLocalViewingPlayerController` _player) (`SceneComponent.K2_GetComponentRotation` _dialoguecamera))
      (bind _returnvalue_2 (`|CreateWidget` "/Game/IkeaBlueprints/Widgets/WB_DialogueCombat.WB_DialogueCombat_C" (`GameplayStatics.GetPlayerController` 0)))
      (`UserWidget.AddToViewport` _returnvalue_2 0)
      (`WidgetBlueprintLibrary.SetInputMode_UIOnlyEx` _returnvalue null "LockAlways")
      (set `PlayerController.bShowMouseCursor` true _returnvalue)
      (`SceneComponent.SetVisibility` (`Character.Mesh` _player_2) false false))))

(event `EndDialogue`
  (bind _returnvalue (`Pawn.GetLocalViewingPlayerController` (`self.Player`)))
  (`CharacterMovementComponent.SetMovementMode` (`Character.CharacterMovement` (`self.Player`)) "MOVE_Falling" 0)
  (`self.SetActive` (`/Game/ThirdPerson/Blueprints/BP_ThirdPersonCharacter.FollowCamera` (`self.Player`)) true false)
  (`self.SetActive` (`/Game/StealthAI/EnemyAI/BP_EnemyAI_PARENT.DialogueCamera` (`self.ThisEnemy`)) false false)
  (`WidgetBlueprintLibrary.SetInputMode_GameOnly` _returnvalue)
  (set `PlayerController.bShowMouseCursor` false _returnvalue)
  (`SceneComponent.SetVisibility` (`Character.Mesh` (`self.Player`)) true false))

(event `UpdateDialogue`)