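; Parent stealth enemy Blueprint that runs a Search, Patrol or Guard behavior tree and exposes guard, patrol and noise data.
; Seeing the player fills a timeline-driven meter, or instantly triggers a chase with music; a retriggerable delay drains or cancels it once sightings stop.
; AI Perception stimuli trigger investigation through Blackboard flags unless chasing.
; It also spawns optionally timed tap-key prompts and exposes combat and health components.
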(event `self.ReceiveBeginPlay`
  (bind _ai_controller_ref (`self.AI Controller REF`))
  (`|ExecutionSequence`
    (:`then_0`
      ;[1 1 1] Set AI type based on dev choice
      (set `self.AI Controller REF` (`AIBlueprintHelperLibrary.GetAIController` self))
      (switch `/Game/StealthAI/GameBlueprints/E_AI_Type` (`self.AI Type`)
        (:`NewEnumerator0`
          (`AIController.RunBehaviorTree` _ai_controller_ref "/Game/StealthAI/EnemyAI/BT/BT_SAI_Search.BT_SAI_Search"))
        (:`NewEnumerator1`
          (`AIController.RunBehaviorTree` _ai_controller_ref "/Game/StealthAI/EnemyAI/BT/BT_SAI_Patrol.BT_SAI_Patrol"))
        (:`NewEnumerator2`
          (`AIController.RunBehaviorTree` (`self.AI Controller REF`) "/Game/StealthAI/EnemyAI/BT/BT_SAI_Guard.BT_SAI_Guard"))))
    (:`then_1`
      ;[1 1 1] Set guard post position
      (set `self.GuardPostPosition` (`KismetMathLibrary.SelectVector` (`self.K2_GetActorLocation`) (`self.GuardPostPosition`) (`self.Use Current Position?`))))
    (:`then_2`
      ;[1 1 1] Set reference to the detection meter widget
      (bind _asw_detection_meter (cast `/Game/StealthAI/UI/W_DetectionMeter` (`WidgetComponent.GetWidget` (`self.Detection Meter`))))
      (set `self.DM Widget` _asw_detection_meter)
      ;[1 1 1] Set the detection time defined by the user
      (`TimelineComponent.SetPlayRate` (`self.Fill Detection Meter`) (/ 1.0 (`self.Detection Time`))))))

(event `self.PawnSensing.OnSeePawn`
  (params (Pawn :type "Pawn Object Reference"))
  (bind _charactermovement (`self.CharacterMovement`))
  (bind _returnvalue (`AIBlueprintHelperLibrary.GetBlackboard` (`self.AI Controller REF`)))
  (bind _progressbar_23 (`/Game/StealthAI/UI/W_DetectionMeter.ProgressBar_23` (`self.DM Widget`)))
  ;[1 1 1] Detect player
  (if (and (== Pawn (`GameplayStatics.GetPlayerCharacter` 0)) (`self.IsDetecting?`))
    (`|ExecutionSequence`
      (:`then_0`
        ;;[1 1 1] Fill up/drain detection meter
        (if (`self.Detect Immediately`)
          ;;[1 1 1] Start chasing
          (`BlackboardComponent.SetValueAsBool` _returnvalue "CanSeePlayer?" true :!label _label)
          (set `CharacterMovementComponent.MaxWalkSpeed` 150.0 _charactermovement)
          ;;[1 1 1] Change colour of meter
          (`ProgressBar.SetFillColorAndOpacity` _progressbar_23 (struct :`R` 1.0 :`A` 1.0))
          (set `self.IsChasing?` true)
          (`/Game/StealthAI/EnemyAI/AC_EnemyCombat.ChaseUpdate` (`self.AC_EnemyCombat`))
          (`/Engine/EditorBlueprintResources/StandardMacros.DoOnce` false :!label _label_2
            (:`Completed`
              (`GameplayStatics.PlaySoundAtLocation` "/Game/StealthAI/SFX/ChaseHey/ChaseHey_CUE.ChaseHey_CUE" (`self.K2_GetActorLocation`) (struct) 1.0 1.0 0.0 null null null null)
              (message `/Game/StealthAI/GameBlueprints/BPI_StealthAI.Start Chase Music` (`GameplayStatics.GetGameInstance`))))
          (else
            (`SceneComponent.SetVisibility` (`self.Detection Meter`) true false)
            (`|ExecutionSequence`
              (:`then_0`
                (bind (_direction _detected_amount) (`Timeline|Fill Detection Meter` :!label _label_3)
                  (:`Update`
                    (set `/Game/StealthAI/UI/W_DetectionMeter.Detected Amount` _detected_amount (`self.DM Widget`)))
                  (:`Finished`
                    (switch `ETimelineDirection` _direction
                      (:`Forward`
                        (goto _label))
                      (:`Backward`
                        (`SceneComponent.SetVisibility` (`self.Detection Meter`) false false :!label _label_4)
                        ;;[1 1 1] Stop chasing
                        (`BlackboardComponent.SetValueAsBool` _returnvalue "CanSeePlayer?" false)
                        (set `CharacterMovementComponent.MaxWalkSpeed` 150.0 _charactermovement)
                        (`ProgressBar.SetFillColorAndOpacity` _progressbar_23 (struct :`R` 1.0 :`G` 1.0 :`B` 1.0 :`A` 1.0))
                        (set `self.IsChasing?` false)
                        (message `/Game/StealthAI/GameBlueprints/BPI_StealthAI.Stop Chase Music` (`GameplayStatics.GetGameInstance`))
                        (goto _label_2 :!via `Reset`))))))
              (:`then_1`
                (`/Engine/EditorBlueprintResources/StandardMacros.DoOnce` false :!label _label_5
                  (:`Completed`
                    (`GameplayStatics.PlaySoundAtLocation` "/Game/StealthAI/SFX/DetectionHuh/DetectionHuh_CUE.DetectionHuh_CUE" (`self.K2_GetActorLocation`) (struct) 1.0 1.0 0.0 null null null null))))))))
      (:`then_1`
        (`KismetSystemLibrary.RetriggerableDelay` (`self.Search Time`))
        (if (`self.Detect Immediately`)
          (goto _label_4)
          (else
            (`TimelineComponent.Stop` (`self.Fill Detection Meter`))
            (`|ExecutionSequence`
              (:`then_0`
                (goto _label_5 :!via `Reset`))
              (:`then_1`
                (goto _label_3 :!via `Reverse`)))))))))

(event `self.AIPerception.OnTargetPerceptionUpdated`
  (params (Actor :type "Actor Object Reference") (Stimulus :type "AIStimulus Structure"))
  (bind ((`StimulusLocation` _stimuluslocation) (`bSuccessfullySensed` _bsuccessfullysensed)) (break `AIStimulus` Stimulus))
  ;[1 1 1] Investigate any noise heard
  (if _bsuccessfullysensed
    (set `self.Noise Location` _stimuluslocation)
    (if (not (`self.IsChasing?`))
      (`BlackboardComponent.SetValueAsBool` (`AIBlueprintHelperLibrary.GetBlackboard` (`self.AI Controller REF`)) "HeardNoise?" true)
      (`GameplayStatics.PlaySoundAtLocation` "/Game/StealthAI/SFX/DetectionHuh/DetectionHuh_CUE.DetectionHuh_CUE" (`self.K2_GetActorLocation`) (struct) 1.0 1.0 0.0 null null null null))))

(event `/Game/StealthAI/GameBlueprints/BPI_StealthAI.EndInvestigation`
  ;[1 1 1] Investigate any noise heard
  (`BlackboardComponent.SetValueAsBool` (`AIBlueprintHelperLibrary.GetBlackboard` (`self.AI Controller REF`)) "HeardNoise?" false))

(event `StartDetectionCooldown`
  (if (not (`self.IsDetecting?`))
    (`KismetSystemLibrary.K2_SetTimer` null "StartDetection" (`self.Detection Cooldown`))))

(event `Create Tap Key Event`
  (params (TargetKey :type "Key Structure" :default "None") (TargetKeyText :type Text) (`IsTimed?` :type Boolean) (Duration :type "Float (double-precision)") (CalledFrom :type "Actor Object Reference"))
  (bind _currtapkeyref (`self.CurrTapKeyRef`))
  ;[1 1 1] Create a tap key event
  (bind _returnvalue (`|CreateWidget` "/Game/IkeaBlueprints/TapKeySystem/WB_TapKeyUI.WB_TapKeyUI_C" (`GameplayStatics.GetPlayerController` 0)))
  (`/Game/IkeaBlueprints/TapKeySystem/WB_TapKeyUI.SetEnemy` _returnvalue self)
  (`UserWidget.AddToViewport` _returnvalue 0)
  (bind _output_get (set `self.CurrTapKeyRef` _returnvalue))
  (set `/Game/IkeaBlueprints/TapKeySystem/WB_TapKeyUI.Key` TargetKey _output_get)
  (set `self.InTapKeyProgress?` true)
  (`/Game/IkeaBlueprints/TapKeySystem/WB_TapKeyUI.Set text` _output_get TargetKeyText)
  (if `IsTimed?`
    (`TimelineComponent.SetPlayRate` (`self.Duration progress bar timeline`) (/ 1.0 Duration))
    (bind (_direction _value) (`Timeline|Duration progress bar timeline` :!via `PlayFromStart`) ; Make sure length is 1.0
      (:`Update`
        (`ProgressBar.SetPercent` (`/Game/IkeaBlueprints/TapKeySystem/WB_TapKeyUI.TimerBar` (`self.CurrTapKeyRef`)) (`KismetMathLibrary.Lerp` 1.0 0.0 _value)))
      (:`Finished`
        ;;[1 0 0] On Failed
        (if (`self.InTapKeyProgress?`)
          (`UserWidget.PlayAnimation` _currtapkeyref (`/Game/IkeaBlueprints/TapKeySystem/WB_TapKeyUI.Failed` _currtapkeyref) 0.0 1 "Forward" 1.0 false))
        (set `/Game/IkeaBlueprints/TapKeySystem/WB_TapKeyUI.TapKeyProgress` 0.0 _currtapkeyref)
        (set `self.InTapKeyProgress?` false)))))

(event `self.K2_OnReset`
  (`/Game/StealthAI/EnemyAI/AC_EnemyCombat.OnReset` (`self.AC_EnemyCombat`)))

(fn `GetCombatComponent`
  (returns (AC_EnemyCombat :type "/Game/StealthAI/EnemyAI/AC_EnemyCombat Object Reference"))
  (return (`self.AC_EnemyCombat`)))

(fn `GetGuardPost`
  (returns (Location :type "Vector Structure"))
  (return (`self.GuardPostPosition`)))

(fn `GetHealthComponent`
  (returns (AC_HealthComponent :type "/Game/IkeaBlueprints/Components/AC_HealthComponent Object Reference"))
  (return (`self.AC_HealthComponent`)))

(fn `GetNoiseLocation`
  (returns (Location :type "Vector Structure"))
  (return (`self.Noise Location`)))

(fn `GetpatrolPoints`
  (returns (`Patrol Path` :type "Array of /Game/StealthAI/EnemyAI/BP_PatrolPoint Object Reference"))
  ;[1 1 1] Get the patrol points on the desired patrol path
  (bind _outactors (`GameplayStatics.GetAllActorsOfClass` "/Game/StealthAI/EnemyAI/BP_PatrolPoint.BP_PatrolPoint_C"))
  (for _array_element _outactors
    (if (== (`/Game/StealthAI/EnemyAI/BP_PatrolPoint.Patrol Path Index` _array_element) (`self.Patrol Path Index`))
      (`KismetArrayLibrary.Array_Add` (`self.Patrol Path`) _array_element)))
  (return (`self.Patrol Path`)))

(fn `StartDetection`
  (set `self.IsDetecting?` true))

(fn `StopDetection`
  (set `self.IsDetecting?` false))

(fn `UserConstructionScript`)