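; BP_PatrolPoint is a patrol point marker for enemy AI in a stealth setup, carrying a path index and an arrow.
; Its construction script sizes the arrow and both text labels from exposed variables and applies a shared colour to the labels.
; The path label shows the patrol path index, so points read clearly when placed in the level.
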(fn `UserConstructionScript`
  (bind _path_text (`self.Path Text`))
  (bind _text_size (`self.Text Size`))
  ;[1 1 1] Update arrow and text size, as well as text content and colour
  (set `ArrowComponent.ArrowSize` (`self.Arrow Size`) (`self.Arrow`))
  (`TextRenderComponent.SetXScale` _path_text _text_size)
  (`TextRenderComponent.SetXScale` (`self.Order Text`) _text_size)
  (`TextRenderComponent.SetYScale` _path_text _text_size)
  (`TextRenderComponent.SetYScale` (`self.Order Text`) _text_size)
  (`TextRenderComponent.K2_SetText` _path_text (`|FormatText` "Path: {Path}" (`KismetTextLibrary.Conv_IntToText` (`self.Patrol Path Index`))))
  (`TextRenderComponent.SetTextRenderColor` (`self.Order Text`) (`self.Path Text Colour`))
  (`TextRenderComponent.SetTextRenderColor` (`self.Path Text`) (`self.Path Text Colour`)))